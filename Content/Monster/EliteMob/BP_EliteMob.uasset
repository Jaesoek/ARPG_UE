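; BP_EliteMob is an elite monster actor, with most of its gameplay logic not present in these graphs.
; Every Tick turns its HP bar widget in world space toward the first player's pawn, billboard style.
; BeginPlay binds a take-any-damage handler that is currently empty.
; The e_Notify event adds a widget component without using its NotifyWidget input, and the construction script is empty.
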(event `e_Notify`
  (params (NotifyWidget :type "UserWidget Object Reference"))
  (`AddComponent|NODE_AddWidgetComponent-0`))

(event `OnTakeAnyDamage_Event_0` :!signature `self.OnTakeAnyDamage`
  (params (DamagedActor :type "Actor Object Reference") (Damage :type "Float (double-precision)") (DamageType :type "DamageType Object Reference") (InstigatedBy :type "Controller Object Reference") (DamageCauser :type "Actor Object Reference")))

(event `self.ReceiveBeginPlay`
  (add `self.OnTakeAnyDamage` (delegate `OnTakeAnyDamage_Event_0`)))

(event `self.ReceiveTick`
  (params (DeltaSeconds :type "Float (single-precision)"))
  ;[1 1 1] HpBar - Rotate to Player
  (`SceneComponent.K2_SetWorldRotation` (`self.m_HpBarWidget`) (`KismetMathLibrary.Conv_VectorToRotator` (- (`self.K2_GetActorLocation` (`Controller.K2_GetPawn` (`GameplayStatics.GetPlayerController` 0))) (`self.K2_GetActorLocation`))) false false))

(fn `UserConstructionScript`)