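; Trash mob monster Blueprint that animates an erode effect on its mesh over about the first second after spawning.
; BeginPlay creates a dynamic material instance from the mesh's first material slot and resets its "erode" scalar to zero.
; Tick accumulates delta time into MMeshOpacity and writes it to "erode" while it stays at or below one, though the counter keeps growing afterward.
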(event `self.ReceiveTick`
  (params (DeltaSeconds :type "Float (single-precision)"))
  (bind _output_get (set `self.m_MeshOpacity` (+ DeltaSeconds (`self.m_MeshOpacity`))))
  (if (<= _output_get 1.0)
    (`MaterialInstanceDynamic.SetScalarParameterValue` (`self.m_MID_Mesh`) "erode" _output_get)))

(event `self.ReceiveBeginPlay`
  (bind _mesh (`self.Mesh`))
  (bind _returnvalue (`PrimitiveComponent.CreateDynamicMaterialInstance` _mesh 0 (`PrimitiveComponent.GetMaterial` _mesh 0) "None"))
  (bind _output_get (set `self.m_MID_Mesh` _returnvalue))
  (bind _output_get_2 (set `self.m_MeshOpacity` 0.0))
  (`MaterialInstanceDynamic.SetScalarParameterValue` _output_get "erode" _output_get_2))

(fn `UserConstructionScript`)